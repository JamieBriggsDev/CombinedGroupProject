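; Game instance that runs menu flow, player profile loading and multiplayer session handling.
; It checks for a saved profile to open the main or options menu, reusing cached widgets except the server menu, which is created fresh.
; It creates or joins sessions behind a loading screen, opening LobbyMap as a listen server when hosting.
; Session, network and travel failures feed an error dialog; it also stores team data and forwards respawns to TeamDeathmatchIns.
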(event Custom|ShowMainMenu
  (bind _returnvalue (Game|GetPlayerController 0))
  ;[1 1 1] Shows the main menu
  (CallFunction|LoadGame)
  (Utilities|IsValid (Variables|Widgets|GetMainMenuWB)
    (:Is%20Valid
      _)
    (:Is%20Not%20Valid
      (bind _returnvalue_2 (UserInterface|CreateWidget "/Game/UI/MainMenu/MainMenu.MainMenu_C" _returnvalue))
      (Variables|Widgets|SetMainMenuWB _returnvalue_2)))
  (UserInterface|Viewport|AddtoViewport (Variables|Widgets|GetMainMenuWB) 0)
  (Variables|/Script/Engine.PlayerController|SetbShowMouseCursor _returnvalue true)
  (Default|UpdateVariables (Variables|Widgets|GetMainMenuWB) (Variables|Default|GetPlayerInfo)))

(event Custom|StorePlayerData
  (params (_teamBlue :type Team%20Info%20Structure) (_teamRed :type Team%20Info%20Structure))
  (Variables|InGame|SetTeamBlue _teamBlue)
  (Variables|InGame|SetTeamRed _teamRed))

(event Custom|ShowLoadingScreen
  ;[1 1 1] Show loading screen
  (Utilities|IsValid (Variables|Widgets|GetLoadingScreenWB)
    (:Is%20Valid
      _)
    (:Is%20Not%20Valid
      (bind _returnvalue (UserInterface|CreateWidget "/Game/UI/Misc/LoadingScreen.LoadingScreen_C" (Game|GetPlayerController 0)))
      (Variables|Widgets|SetLoadingScreenWB _returnvalue)))
  (UserInterface|Viewport|AddtoViewport (Variables|Widgets|GetLoadingScreenWB) 0))

(event Custom|JoinServer
  (params (_sessionToJoin :type Blueprint%20Session%20Result%20Structure))
  ;[1 1 1] Join Server
  (CallFunction|ShowLoadingScreen)
  (|JoinSession (Game|GetPlayerController 0) _sessionToJoin
    (:OnFailure
      (Utilities|DisplayErrorMessage "FAILED TO JOIN SESSION. PLEASE TRY AGAIN."))))

(event Custom|ShowServerMenu
  ;[1 1 1] Show the server menu, creates a new one each time it is called
  (bind _returnvalue (UserInterface|CreateWidget "/Game/UI/MainMenu/ServerMenu.ServerMenu_C" (Game|GetPlayerController 0)))
  (UserInterface|Viewport|AddtoViewport _returnvalue 0))

(event Custom|ShowOptionsMenu
  ;[1 1 1] Shows the options menu
  (Utilities|IsValid (Variables|Widgets|GetOptionsMenuWB)
    (:Is%20Valid
      _)
    (:Is%20Not%20Valid
      (bind _returnvalue (UserInterface|CreateWidget "/Game/UI/MainMenu/OptionsMenu.OptionsMenu_C" (Game|GetPlayerController 0)))
      (Variables|Widgets|SetOptionsMenuWB _returnvalue)))
  (UserInterface|Viewport|AddtoViewport (Variables|Widgets|GetOptionsMenuWB) 0))

(event Custom|DestroySessionCaller
  (params (_playerController :type Player%20Controller%20Object%20Reference))
  ;[1 1 1] Destroy Session when called
  (|DestroySession _playerController))

(event Custom|CheckSaveGame
  ;[1 1 1] Check for save game
  (bind _returnvalue (SaveGame|DoesSaveGameExist (Variables|Default|GetPlayerProfileSave)))
  (if _returnvalue
    (CallFunction|ShowMainMenu)
    (CallFunction|LoadGame)
    (Default|UpdateVariables (Variables|Widgets|GetMainMenuWB) (Variables|Default|GetPlayerInfo))
    (Variables|Default|SetCreatedSaveFile true)
    (else
      (CallFunction|ShowOptionsMenu)
      (Variables|/Script/Engine.PlayerController|SetbShowMouseCursor (Game|GetPlayerController 0) true))))

(event Custom|LaunchLobby
  (params (_numberOfPlayers :type Integer) (_enableLan :type Boolean) (_serverName :type Text))
  ;[1 1 1] Launch The Lobby
  (Variables|ServerSettings|SetMaxPlayers _numberOfPlayers)
  (Variables|ServerSettings|SetIsLan _enableLan)
  (Variables|ServerSettings|SetServerName _serverName)
  (CallFunction|ShowLoadingScreen)
  (|Session (Game|GetPlayerController 0) (Variables|ServerSettings|GetMaxPlayers) (Variables|ServerSettings|GetIsLan)
    (:OnSuccess
      (Game|OpenLevel(byName) "LobbyMap" true "listen"))
    (:OnFailure
      (Utilities|DisplayErrorMessage "FAILED TO CREATE SESSIONS, PLEASE TRY AGAIN."))))

(event Custom|ShowHostMenu
  ;[1 1 1] Shows the host game menu
  (Utilities|IsValid (Variables|Widgets|GetHostMenuWB)
    (:Is%20Valid
      _)
    (:Is%20Not%20Valid
      (bind _returnvalue (UserInterface|CreateWidget "/Game/UI/MainMenu/HostMenu.HostMenu_C" (Game|GetPlayerController 0)))
      (Variables|Widgets|SetHostMenuWB _returnvalue)))
  (UserInterface|Viewport|AddtoViewport (Variables|Widgets|GetHostMenuWB) 0))

(event Custom|RespawnGamePlay
  (params (Controller :type Gameplay%20PC%20Object%20Reference))
  (Default|RespawnPlayer (Variables|Default|GetTeamDeathmatchIns) Controller (.PlayerCharacter (Utilities|Struct|BreakPlayerInfo (Variables|/Game/Blueprints/Gameplay/GameplayPC.GameplayPC_C|GetPlayerSettings Controller)))))

(event EventHandleNetworkError
  (params (FailureType :type ENetworkFailure%20Enum :default "NetDriverAlreadyExists") (bIsServer :type Boolean))
  ;[1 1 1] Handle Network Errors and show message
  (if bIsServer
    _
    (else
      _))
  (Utilities|DisplayErrorMessage (CallFunction|NetworkErrortoString FailureType)))

(event EventHandleTravelError
  (params (FailureType :type ETravelFailure%20Enum :default "NoLevel"))
  ;[1 1 1] Handle Travel Errors and show message
  (Utilities|DisplayErrorMessage (CallFunction|TravelErrortoString FailureType)))

(fn NetworkErrortoString
  (params (_failType :type ENetworkFailure%20Enum :default "NetDriverAlreadyExists"))
  (switch Utilities|FlowControl|Switch|SwitchonENetworkFailure _failType
    (:NetDriverAlreadyExists
      (Variables|Default|SetErrorString "Errror - Lost Connection to Host" :!label _label))
    (:NetDriverCreateFailure
      (goto _label))
    (:NetDriverListenFailure
      (goto _label))
    (:ConnectionLost
      (goto _label))
    (:ConnectionTimeout
      (Variables|Default|SetErrorString "Errror - Connection Timed Out"))
    (:FailureReceived
      (goto _label))
    (:OutdatedClient
      (goto _label))
    (:OutdatedServer
      (goto _label))
    (:PendingConnectionFailure
      (goto _label))
    (:NetGuidMismatch
      (goto _label))
    (:NetChecksumMismatch
      (goto _label)))
  (return (Variables|Default|GetErrorString)))

(fn TravelErrortoString
  (params (_failureType :type ETravelFailure%20Enum :default "NoLevel"))
  (return (Utilities|String|Append "Error - Failed to travel. " (Utilities|String|EnumtoString _failureType))))

(fn LoadGame
  (bind _returnvalue (SaveGame|LoadGamefromSlot (Variables|Default|GetPlayerProfileSave)))
  (bind _asplayer_save_game (Utilities|Casting|CastToPlayerSaveGame _returnvalue))
  (Variables|Default|SetPlayerInfo (Variables|/Game/Blueprints/Global/PlayerSaveGame.PlayerSaveGame_C|GetS_PlayerInfo _asplayer_save_game)))