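; AI controller for shooter bots that runs their behavior tree and handles combat.
; BeginPlay sets up the blackboard with the spawn point as HomeLocation; Tick calls Shoot, which fires at and pitches toward the bot's living enemy.
; PassBotInfoToServer registers the bot with the game mode and team, then respawns it.
; Random-name setup via SetBotInfo is disconnected, and FindClosestEnemyWithLOS is an unfinished stub.
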(event Custom|Shoot
  ;[1 1 1] Tells bot to shoot
  (bind _assk_base_bot (Utilities|Casting|CastToSK_BaseBot (Pawn|GetControlledPawn)))
  (Variables|Shooting|SetCanShoot false)
  (bind _enemy (Default|GetEnemy _assk_base_bot))
  (bind _output_get (Variables|AI|SetEnemyBot _enemy))
  (Utilities|IsValid _output_get
    (:Is%20Valid
      (bind _assk_base (Utilities|Casting|CastToSK_Base _output_get)
        (:then
          (bind _alive (Default|IsAlive _assk_base))
          (if _alive
            (Variables|Shooting|SetCanShoot true :!label _label)
            (Default|FireWeapon _assk_base_bot)
            (CallFunction|FaceLocation (Transformation|GetActorLocation (Variables|AI|GetEnemyBot)))
            (else
              (Default|StopFireWeapon _assk_base_bot :!label _label_2))))
        (:CastFailed
          (bind _assk_base_bot_2 (Utilities|Casting|CastToSK_BaseBot _output_get))
          (bind __isalive (Default|IsAlive _assk_base_bot_2))
          (if __isalive
            (goto _label)
            (else
              (goto _label_2))))))))

(event Custom|StopShoot
  ;[1 1 1] Tells bot to stop shooting
  (bind _assk_base_bot (Utilities|Casting|CastToSK_BaseBot (Pawn|GetControlledPawn)))
  (Default|StopFireWeapon _assk_base_bot))

(event Custom|PassBotInfoToServer
  (params (PlayerSettings :type Player%20Info%20Structure))
  (bind _self self)
  ;[1 1 1] Adds the bot to the game mode
  (Variables|AI|SetPlayerSettings PlayerSettings)
  (bind _asgameplay_gm (Utilities|Casting|CastToGameplayGM (Game|GetGameMode)))
  (Utilities|Array|Add (Variables|/Game/Blueprints/Gameplay/GameplayGM.GameplayGM_C|GetPlayerInfo _asgameplay_gm) (Variables|AI|GetPlayerSettings))
  (bind _asteam_death_match (Utilities|Casting|CastToTeamDeathMatch _asgameplay_gm))
  (Default|AddBotTeamMember _asteam_death_match _self)
  (Default|RespawnBot _asgameplay_gm _self (.PlayerCharacter (Utilities|Struct|BreakPlayerInfo (Variables|AI|GetPlayerSettings))) (Variables|AI|GetBotName)))

(event EventBeginPlay
  ;[1 1 1] Sets up bot by setting up blackboard and giving the bot a random name
  (Class|AIController|UseBlackboard "/Game/Blueprints/Bots/AI/BotBB.BotBB")
  (AI|Components|Blackboard|SetValueasVector (AI|GetBlackboard self) (Variables|AI|GetHomeLocation) (Transformation|GetActorLocation (Pawn|GetControlledPawn)))
  (AI|RunBehaviorTree "/Game/Blueprints/Bots/AI/BotBT.BotBT"))

(event EventTick
  (params (DeltaSeconds :type Float%20%28single-precision%29))
  (CallFunction|Shoot))

(fn ConstructionScript)

(fn FindClosestEnemywithLOS
  (params (ExcludedCharacters :type Character%20Object%20Reference))
  (LocalVariables|SetExcludedCharacter ExcludedCharacters)
  (bind _output_get (LocalVariables|SetMyBot (Pawn|GetControlledPawn self)))
  (Utilities|IsValid _output_get
    (:Is%20Valid
      (LocalVariables|SetMyBotLocation (Transformation|GetActorLocation (LocalVariables|GetMyBot)))
      (bind _outactors (Actor|GetAllActorsOfClass "/Script/Engine.Character"))
      (for _array_element _outactors
        (bind _output_get_2 (LocalVariables|SetTestPawn _array_element))
        (bind _assk_base (Utilities|Casting|CastToSK_Base _output_get_2))
        (Utilities|IsValid _assk_base
          (:Is%20Valid
            (if (!= (LocalVariables|GetExcludedCharacter) (LocalVariables|GetTestPawn))
              (bind _alive (Default|IsAlive _assk_base))
              (if _alive
                _))))))))

(fn FaceLocation
  (params (Location :type Vector))
  (Transformation|SetActorRotation (Pawn|GetControlledPawn) (Math|Rotator|MakeRotator 0.0 (.Pitch (Math|Rotator|BreakRotator (Math|Rotator|FindLookatRotation (Transformation|GetActorLocation) Location))) 0.0)))

(fn SetBotInfo
  (params (Character :type Character%20Class%20Reference))
  (bind _returnvalue (Utilities|GetDataTableRow "/Game/Blueprints/Bots/Names.Names" (Utilities|String|StringToName (Utilities|String|ToString(Integer) (Math|Random|RandomInteger 249))))
    (:then
      (Variables|AI|SetPlayerSettings (Utilities|Struct|MakePlayerInfo (Utilities|Text|ToText(String) (Utilities|Struct|BreakNameStructure _returnvalue)) "/Game/Player/AnimStarterPack/UE4_Mannequin/Textures/UE4_LOGO_CARD.UE4_LOGO_CARD" Character 0 "Not Ready!")))))