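; Behavior tree decorator for bots that checks whether the controlled pawn is at the acceptance distance from its follow target.
; It casts the owner to BotAIController, reads the TargetToFollow actor from the blackboard and measures the distance between the two locations.
; The condition uses exact equality with AcceptanceDistance, so it passes only at precisely that distance, not anywhere within it.
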(fn PerformConditionCheck
  (params (OwnerActor :type Actor%20Object%20Reference))
  (bind _asbot_aicontroller (Utilities|Casting|CastToBotAIController OwnerActor))
  (Variables|Default|SetAI_Con_Ref _asbot_aicontroller)
  (return (== (Math|Vector|VectorLength (- (Transformation|GetActorLocation (AI|BehaviorTree|GetBlackboardValueasActor (Variables|Default|GetTargetToFollow))) (Transformation|GetActorLocation (Pawn|GetControlledPawn (Variables|Default|GetAI_Con_Ref))))) (Variables|Default|GetAcceptanceDistance))))