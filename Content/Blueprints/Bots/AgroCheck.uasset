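; AgroCheck is a behavior tree tick node, likely a service, that handles bot aggro.
; Each tick it sphere-traces for desired object types around the pawn of a cached BotAIController, with persistent debug drawing, ignoring all BotAIController actors.
; Each hit gets a Camera-channel line-of-sight trace that writes TargetToFollow and TargetLocation, or clears TargetToFollow when blocked.
; The loop never breaks, so the last hit decides the target.
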(event EventTick
  (params (OwnerActor :type Actor%20Object%20Reference) (DeltaSeconds :type Float%20%28single-precision%29))
  ;[1 1 1] Deals with AI Agro, owner actor is passed in as the controller calling the behaviour tree, does a multi sphere trace for all objects based around the AI without the bot running the process, checks if anyone was hit, if so does a line trace for line of sight then set to follow.
  (if (!= (Variables|Default|GetAI%20Con%20Ref) 0)
    _
    (else
      (bind _asbot_aicontroller (Utilities|Casting|CastToBotAIController OwnerActor))
      (Variables|Default|SetAI%20Con%20Ref _asbot_aicontroller)))
  (bind _outactors (Actor|GetAllActorsOfClass "/Game/Blueprints/Bots/BotAIController.BotAIController_C"))
  (Variables|Default|SetMyLocation (Transformation|GetActorLocation (Pawn|GetControlledPawn (Variables|Default|GetAI%20Con%20Ref))))
  (bind _outhits (Collision|MultiSphereTraceForObjects (Transformation|GetActorLocation (Pawn|GetControlledPawn (Variables|Default|GetAI%20Con%20Ref))) (+ (Transformation|GetActorLocation (Pawn|GetControlledPawn (Variables|Default|GetAI%20Con%20Ref))) "0, 0,15.000000") 1.5e+03 (Variables|Default|GetDesiredObjectTypes) false _outactors "Persistent"))
  (bind _array_element (Utilities|Array|ForEachLoopwithBreak _outhits)
    (:LoopBody
      (bind _outhit (Collision|LineTraceByChannel (Variables|Default|GetMyLocation) (Transformation|GetActorLocation (.HitActor (Collision|BreakHitResult _array_element))) "TraceTypeQuery2" false _outactors "None"))
      (if (== (.HitActor (Collision|BreakHitResult _outhit)) (.HitActor (Collision|BreakHitResult _array_element)))
        (Class|BTFunctionLibrary|SetBlackboardValueasObject (Variables|Default|GetTargetToFollow) (.HitActor (Collision|BreakHitResult _outhit)))
        (AI|BehaviorTree|SetBlackboardValueasVector (Variables|Default|GetTargetLocation) (Transformation|GetActorLocation (.HitActor (Collision|BreakHitResult _outhit))))
        (else
          (Class|BTFunctionLibrary|SetBlackboardValueasObject (Variables|Default|GetTargetToFollow)))))))