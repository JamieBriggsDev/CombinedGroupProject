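; Behavior tree task that moves a bot's controlled pawn to the actor stored in the TargetToFollow blackboard key.
; It casts the owner to BotAIController on first use and caches it for later executions.
; AIMoveTo runs with a small acceptance radius, and the task finishes successfully on arrival.
; A failed move or failed cast never calls FinishExecute.
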(event EventReceiveExecute
  (params (OwnerActor :type Actor%20Object%20Reference))
  (if (!= (Variables|Default|GetAI_Con_Ref) 0)
    _
    (else
      (bind _asbot_aicontroller (Utilities|Casting|CastToBotAIController OwnerActor))
      (Variables|Default|SetAI_Con_Ref _asbot_aicontroller)))
  (AI|AIMoveTo (Pawn|GetControlledPawn (Variables|Default|GetAI_Con_Ref)) "0, 0, 0" (AI|BehaviorTree|GetBlackboardValueasActor (Variables|Default|GetTargetToFollow)) 5e+01 false
    (:OnSuccess
      (AI|BehaviorTree|FinishExecute true))))