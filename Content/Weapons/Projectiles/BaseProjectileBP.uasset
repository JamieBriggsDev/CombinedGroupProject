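; Base projectile Blueprint for weapons that explodes into an impact effect and leaves paint where it hits.
; It sets a ten-second lifespan on BeginPlay so stray shots clean themselves up.
; When the Bullet component hits, it spawns an emitter and sound at the impact point and destroys itself.
; It also places a long-lived paint decal oriented along the surface normal.
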(event OnComponentHit(Bullet)
  (params (HitComponent :type Primitive%20Component%20Object%20Reference) (OtherActor :type Actor%20Object%20Reference) (OtherComp :type Primitive%20Component%20Object%20Reference) (NormalImpulse :type Vector :default "0, 0, 0") (Hit :type Hit%20Result%20Structure%20%28by%20ref%29))
  (bind (_bblockinghit _binitialoverlap _time _distance _location _impactpoint _normal _impactnormal) (Collision|BreakHitResult Hit))
  (Effects|SpawnEmitteratLocation (Variables|Components|GetImpactEffect) _impactpoint (Transformation|GetActorRotation))
  (Audio|PlaySoundatLocation (Variables|Components|GetImpactSound) _impactpoint "0, 0, 0" 0.1 2.0)
  (Actor|DestroyActor)
  (Rendering|Decal|SpawnDecalatLocation "/Game/Weapons/Paint/Paint.Paint" "15.000000,15.000000,15.000000" _impactpoint (Math|Conversions|RotationFromXVector _impactnormal) 1.5e+02))

(event EventBeginPlay
  (Actor|SetLifeSpan 1e+01))

(event Collision|EventActorBeginOverlap
  (params (OtherActor :type Actor%20Object%20Reference)))

(event EventTick
  (params (DeltaSeconds :type Float%20%28single-precision%29)))

(fn ConstructionScript)