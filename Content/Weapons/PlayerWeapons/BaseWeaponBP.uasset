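; Base player weapon Blueprint that defines empty FireWeapon and StopFireWeapon events and provides shared aiming logic.
; SetCamera stores the character camera used for aiming.
; CalculateShootInfo line-traces forward from that camera with debug drawing, then stores a ShootInfo transform at the muzzle socket, rotated toward the impact point or the trace end on a miss, so shots converge on the view center.
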(event Custom|FireWeapon)

(event Custom|StopFireWeapon)

(event Custom|CalculateShootInfo
  (bind _charactercamera (Variables|Default|GetCharacterCamera))
  (bind _weaponmesh (Variables|Default|GetWeaponMesh))
  (bind _returnvalue (Transformation|GetWorldLocation _charactercamera))
  (bind _returnvalue_2 (Math|Vector|GetForwardVector _charactercamera))
  (bind _returnvalue_3 (Transformation|GetSocketLocation _weaponmesh "Muzzle"))
  (bind _returnvalue_4 (* _returnvalue_2 1e+04))
  (bind _returnvalue_5 (+ _returnvalue _returnvalue_4))
  (bind (_outhit _returnvalue_6) (Collision|LineTraceByChannel _returnvalue _returnvalue_5 "TraceTypeQuery3" false 0 "ForDuration" true "(R=1.000000,G=0.958333,B=0.958333,A=1.000000)"))
  (if _returnvalue_6
    (Variables|Default|SetShootInfo (Math|Transform|MakeTransform _returnvalue_3 (Math|Rotator|FindLookatRotation _returnvalue_3 (.ImpactPoint (Collision|BreakHitResult _outhit)))))
    (else
      (Variables|Default|SetShootInfo (Math|Transform|MakeTransform _returnvalue_3 (Math|Rotator|FindLookatRotation _returnvalue_3 _returnvalue_5))))))

(event EventBeginPlay)

(event Collision|EventActorBeginOverlap
  (params (OtherActor :type Actor%20Object%20Reference)))

(event EventTick
  (params (DeltaSeconds :type Float%20%28single-precision%29)))

(fn ConstructionScript)

(fn SetCamera
  (params (_camera :type Camera%20Component%20Object%20Reference))
  (Variables|Default|SetCharacterCamera _camera))